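; BP_PlayerCharacter is the player character Blueprint, handling projectile shooting through Enhanced Input.
; When IA_Shoot starts, it asks CombatComponent to spend shot energy and, on success, spawns BP_PlayerProjectile_Base at MuzzleOffset's world location and rotation with itself as instigator.
; Every Tick, it writes CombatComponent's IsAttacking state to DebugText.
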(event `self.ReceiveTick`
  (params (DeltaSeconds :type "Float (single-precision)"))
  (`TextRenderComponent.K2_SetText` (`self.DebugText`) (`KismetTextLibrary.Conv_BoolToText` (`JSCombatComponent.IsAttacking` (`self.CombatComponent`)))))

(event `EnhancedInput|/Game/Input/IA_Shoot`
  (params (ActionValue :type Boolean) (ElapsedSeconds :type "Float (double-precision)") (TriggeredSeconds :type "Float (double-precision)") (InputAction :type "InputAction Object Reference" :default "/Game/Input/IA_Shoot.IA_Shoot"))
  (bind _muzzleoffset (`self.MuzzleOffset`))
  (:`Started`
    (bind _returnvalue (`JSCombatComponent.SpendShotEnergy` (`self.CombatComponent`) 1.0))
    (if _returnvalue
      (`|SpawnActorFromClass` "/Game/Blueprints/Projectiles/Player/BP_PlayerProjectile_Base.BP_PlayerProjectile_Base_C" (`KismetMathLibrary.MakeTransform` (`SceneComponent.K2_GetComponentLocation` _muzzleoffset) (`SceneComponent.K2_GetComponentRotation` _muzzleoffset)) "AlwaysSpawn" "MultiplyWithRoot" null self))))

(fn `UserConstructionScript`)